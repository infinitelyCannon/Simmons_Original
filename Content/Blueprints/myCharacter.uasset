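; Player character for a programming-themed puzzle game: spawns logic gates on nodes, teleports and kills viruses to reach the level end.
; Tick line-traces from screen center to pick viruses, teleport points or spawn nodes, highlighted with debug shapes; input events act on that target.
; External calls unlock teleport and kill, or end the level, which reloads Main.
; It also drives HUD messages, gate cycling, pause, unlit view and ASCII-effect monochrome toggles.
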(event EventBeginPlay
  (bind _outactors (Actor|GetAllActorsOfClass "/Game/Blueprints/AsciiVolume.AsciiVolume_C"))
  (if (> (Utilities|Array|Length _outactors) 0)
    _
    (else
      _))
  (Variables|Default|SetAsciiEffect (Utilities|Array|Get(acopy) _outactors))
  (bind _asmuh_hud (Utilities|Casting|CastTomuhHUD (HUD|GetHUD (Game|GetPlayerController 0))))
  (bind _output_get (Variables|Default|SetLogWidget (Variables|/Game/Widgets/muhHUD.muhHUD_C|GetWidgetRef _asmuh_hud)))
  (Default|ShowMessage _output_get "(R=1.000000,G=1.000000,B=1.000000,A=1.000000)" 1e+01 "Welcome! Make your way to the end by unlocking the logical gates. 
Press \"E\" when looking at a \"?\" node to spawn a gate. 
Press \"Q\" to toggle color.")
  (Development|PrintString "Welcome! Make your way to the end by unlocking the logical gates. 
Press \"E\" when looking at a \"?\" node to spawn a gate. 
Press \"Q\" to toggle color." false))

(event Collision|EventActorBeginOverlap
  (params (OtherActor :type Actor%20Object%20Reference)))

(event EventTick
  (params (DeltaSeconds :type Float%20%28single-precision%29))
  (bind _returnvalue (Viewport|GetViewportSize))
  (bind _returnvalue_2 (Viewport|GetViewportSize))
  (bind _returnvalue_3 (Game|GetPlayerController 0))
  (bind _array (Utilities|Array|MakeArray "ObjectTypeQuery1" "ObjectTypeQuery2" "ObjectTypeQuery3"))
  (bind _camera (Variables|Default|GetCamera))
  (bind _camera_2 (Variables|Default|GetCamera))
  (bind _raydist (Variables|Default|GetRayDist))
  (bind _returnvalue_4 (/ (.x _returnvalue_2) 2.0))
  (bind _returnvalue_5 (/ (.y _returnvalue_2) 2.0))
  (bind _returnvalue_6 (Math|Vector|GetForwardVector _camera_2))
  (bind _returnvalue_7 (Transformation|GetWorldLocation _camera_2))
  (bind _worldposition (Class|GameplayStatics|DeprojectScreentoWorld _returnvalue_3 (Math|Vector2D|MakeVector2D _returnvalue_4 _returnvalue_5)))
  (bind _returnvalue_8 (* _returnvalue_6 _raydist))
  (bind _returnvalue_9 (+ _returnvalue_7 _returnvalue_8))
  (if (Variables|Default|GetkillAim)
    (bind _outhit (Collision|LineTraceForObjects (.WorldPosition (Class|GameplayStatics|DeprojectScreentoWorld (Game|GetPlayerController 0) (Math|Vector2D|MakeVector2D (/ (.x _returnvalue) 2.0) (/ (.y _returnvalue) 2.0)))) (+ (Transformation|GetWorldLocation _camera) (* (Math|Vector|GetForwardVector _camera) (Variables|Default|GetRayDist))) (Utilities|Array|MakeArray "ObjectTypeQuery1" "ObjectTypeQuery2" "ObjectTypeQuery3") false 0 "None"))
    (bind _asvirus (Utilities|Casting|CastToVirus (.hitactor _outhit)))
    (bind _output_get (Variables|Default|SetvirusRef _asvirus))
    (Rendering|Debug|DrawDebugSphere (Transformation|GetActorLocation _output_get) 1.5e+02 24 "(R=1.000000,G=1.000000,B=1.000000,A=1.000000)" 0.02)
    (else
      (if (Variables|Default|GetisAiming)
        (bind (_outhit_2 _returnvalue_10) (Collision|LineTraceForObjects _worldposition _returnvalue_9 _array false 0 "None"))
        (if _returnvalue_10
          (bind _output_get_2 (Variables|Default|SetSpawnVec (.location _outhit_2)))
          (Rendering|Debug|DrawDebugSphere _output_get_2 5e+01 24 "(R=1.000000,G=0.200192,B=0.000000,A=1.000000)" 0.02 15.0)
          (else
            (Variables|Default|SetSpawnVec "0, 0, 0")))
        (else
          (Variables|Default|SetSpawnVec "0, 0, 0")
          (bind _outhit_3 (Collision|LineTraceForObjects _worldposition _returnvalue_9 _array false 0 "None"))
          (bind _asspawn_node (Utilities|Casting|CastToSpawnNode (.hitactor _outhit_3))
            (:then
              (Variables|Default|SetspawnTarget _asspawn_node)
              (Variables|Default|SetcanSpawn true)
              (Rendering|Debug|DrawDebugBox (Transformation|GetActorLocation _asspawn_node) "50.000000,50.000000,50.000000" "(R=1.000000,G=1.000000,B=1.000000,A=1.000000)" "0, 0, 0" 0.02 15.0))
            (:CastFailed
              (Variables|Default|SetcanSpawn false)))))
      (if (Variables|Default|GetshouldEnd)
        (Utilities|FlowControl|DoOnce false
          (:Completed
            (Utilities|FlowControl|Delay 5.2)
            (Game|OpenLevel(byName) "Main")))))))

(event Input|ActionEvents|InputActionTimeTrigger
  (params (Key :type Key%20Structure))
  (:Pressed
    (bind _isa (Utilities|FlowControl|FlipFlop)
      (:A
        _)
      (:B
        _))
    (Default|TogglePause (Variables|Default|GetLogWidget) _isa)
    (Game|SetGamePaused _isa)))

(event Input|ActionEvents|InputActionLitTrigger
  (params (Key :type Key%20Structure))
  (:Pressed
    (Utilities|FlowControl|FlipFlop
      (:A
        (Development|ExecuteConsoleCommand "viewmode unlit" 0))
      (:B
        (Development|ExecuteConsoleCommand "viewmode lit" 0)))))

(event Input|ActionEvents|InputActionRestart
  (params (Key :type Key%20Structure))
  (:Pressed
    (Game|OpenLevel(byName) "Main")))

(event Input|ActionEvents|InputActionJump
  (params (Key :type Key%20Structure))
  (:Pressed
    (Character|Jump)))

(event Input|ActionEvents|InputActionSpawn
  (params (Key :type Key%20Structure))
  (:Pressed
    (if (Variables|Default|GetcanSpawn)
      (Default|Spawn (Variables|Default|GetspawnTarget) (Variables|Default|GetSpawnChoice)))))

(event Input|ActionEvents|InputActionCycleUp
  (params (Key :type Key%20Structure))
  (:Pressed
    (if (>= (+ (Variables|Default|GetSpawnChoice) 1) 3)
      (Variables|Default|SetSpawnChoice 0)
      (else
        (Variables|Default|SetSpawnChoice (+ (Variables|Default|GetSpawnChoice) 1))))
    (Default|ChangeGate (Variables|Default|GetLogWidget) (Variables|Default|GetSpawnChoice))))

(event Input|ActionEvents|InputActionCycleDown
  (params (Key :type Key%20Structure))
  (:Pressed
    (if (< (- (Variables|Default|GetSpawnChoice) 1) 0)
      (Variables|Default|SetSpawnChoice 2)
      (else
        (Variables|Default|SetSpawnChoice (- (Variables|Default|GetSpawnChoice) 1))))
    (Default|ChangeGate (Variables|Default|GetLogWidget) (Variables|Default|GetSpawnChoice))))

(event Input|ActionEvents|InputActionToggleColor
  (params (Key :type Key%20Structure)))

(event Input|ActionEvents|InputActionAim
  (params (Key :type Key%20Structure))
  (:Pressed
    (if (Variables|Default|GetcanAim)
      (Variables|Default|SetisAiming true)))
  (:Released
    (Variables|Default|SetisAiming false)
    (if (!= (Math|Vector|VectorLength (Variables|Default|GetSpawnVec)) 0.0)
      (Transformation|SetActorLocation (- (Variables|Default|GetSpawnVec) (* (Math|Vector|Normalize (- (Variables|Default|GetSpawnVec) (Transformation|GetActorLocation))) (Variables|Default|GetTeleportOffset))) false false)
      (Variables|Default|SetSpawnVec "0, 0, 0"))))

(event Input|ActionEvents|InputActionToggleColor
  (params (Key :type Key%20Structure))
  (:Pressed
    (bind _isa (Utilities|FlowControl|FlipFlop)
      (:A
        _)
      (:B
        _))
    (Variables|/Game/Blueprints/AsciiVolume.AsciiVolume_C|SetMonochrome (Variables|Default|GetAsciiEffect) (not _isa))))

(event Input|ActionEvents|InputActionKillAim
  (params (Key :type Key%20Structure))
  (bind _virusref (Variables|Default|GetvirusRef))
  (:Pressed
    (if (Variables|Default|GetcanKill)
      (Variables|Default|SetkillAim true)))
  (:Released
    (Variables|Default|SetkillAim false)
    (Utilities|IsValid _virusref
      (:Is%20Valid
        (Default|Die _virusref)))))

(event Input|AxisEvents|InputAxisMoveForward
  (params (AxisValue :type Float%20%28single-precision%29))
  (Pawn|Input|AddMovementInput (Transformation|GetActorForwardVector) AxisValue false))

(event Input|AxisEvents|InputAxisMoveRight
  (params (AxisValue :type Float%20%28single-precision%29))
  (Pawn|Input|AddMovementInput (Transformation|GetActorRightVector) AxisValue false))

(event Input|AxisEvents|InputAxisVerticalTilt
  (params (AxisValue :type Float%20%28single-precision%29))
  (Pawn|Input|AddControllerPitchInput AxisValue))

(event Input|AxisEvents|InputAxisHorizontalTurn
  (params (AxisValue :type Float%20%28single-precision%29))
  (Pawn|Input|AddControllerYawInput AxisValue))

(fn ConstructionScript)

(fn TriggerAim
  (Variables|Default|SetcanAim true)
  (Default|ShowMessage (Variables|Default|GetLogWidget) "(R=1.000000,G=1.000000,B=1.000000,A=1.000000)" 7.0 "GoTo Function Unlocked! 
Aim while holding down LMB and release to teleport.")
  (Development|PrintString "GoTo Function Unlocked! 
Aim while holding down LMB and release to teleport." false true "(R=1.000000,G=1.000000,B=1.000000,A=1.000000)"))

(fn End
  (Default|ShowMessage (Variables|Default|GetLogWidget) "(R=1.000000,G=1.000000,B=1.000000,A=1.000000)" 4.0 "Congratulations! 
Level complete.")
  (Development|PrintString "Congratulations! 
Level complete." false true "(R=1.000000,G=1.000000,B=1.000000,A=1.000000)")
  (Variables|Default|SetshouldEnd true))

(fn Type
  (params (Message :type Text))
  (Default|ShowMessage (Variables|Default|GetLogWidget) "(R=1.000000,G=1.000000,B=1.000000,A=1.000000)" 4.0 Message)
  (Development|PrintString (Utilities|String|ToString(Text) Message) false true "(R=1.000000,G=1.000000,B=1.000000,A=1.000000)"))

(fn Unlock
  (Variables|Default|SetcanPass true))

(fn TriggerKill
  (Variables|Default|SetcanKill true)
  (Default|ShowMessage (Variables|Default|GetLogWidget) "(R=1.000000,G=1.000000,B=1.000000,A=1.000000)" 8.0 "Kill Process Unlocked! 
Use RMB while highlighting a virus to remove it."))