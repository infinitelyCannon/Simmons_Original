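; Password gatekeeper actor that controls access to the upper level by guarding a gate.
; Its static mesh spins continuously on the roll axis in Tick, scaled by delta time.
; When a myCharacter overlaps the box trigger, it checks the character's CanPass flag and reports the result through the character's Type function.
; Granted access destroys the MGate actor, while denied access shows an admin password message.
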(event OnComponentBeginOverlap(Box)
  (params (OverlappedComponent :type Primitive%20Component%20Object%20Reference) (OtherActor :type Actor%20Object%20Reference) (OtherComp :type Primitive%20Component%20Object%20Reference) (OtherBodyIndex :type Integer) (bFromSweep :type Boolean) (SweepResult :type Hit%20Result%20Structure%20%28by%20ref%29))
  (bind _asmy_character (Utilities|Casting|CastTomyCharacter OtherActor))
  (if (not (Variables|/Game/Blueprints/myCharacter.myCharacter_C|GetcanPass _asmy_character))
    (Default|Type _asmy_character "Access Denied: Admin password required for upper level access")
    (else
      (Default|Type _asmy_character "Access Granted")
      (Actor|DestroyActor (Variables|Default|GetmGate)))))

(event EventBeginPlay)

(event Collision|EventActorBeginOverlap
  (params (OtherActor :type Actor%20Object%20Reference)))

(event EventTick
  (params (DeltaSeconds :type Float%20%28single-precision%29))
  (Transformation|AddLocalRotation (Variables|Default|GetStaticMesh) (* (Math|Rotator|MakeRotator -2e+01 0.0 0.0) DeltaSeconds) false false))

(fn ConstructionScript)