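; GuideArrow is an actor that shows an arrow widget which turns green when the game's stage matches its own Stage and red otherwise.
; On BeginPlay it creates the Arrow widget for its widget component, binds ChangeColor to the game mode's stage update event and applies an initial stage.
; The construction script sets a square draw size from Size, and a separate SetColor function allows arbitrary tinting.
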(event Custom|ChangeColor
  (params (Stage :type PlayerStage%20Enum :default "NewEnumerator0"))
  (bind _arrowref (Variables|Default|GetArrowRef))
  (if (Utilities|Enum|Equal(Enum) Stage (Variables|Widget|GetStage))
    (Default|SetColor _arrowref (Utilities|Struct|MakeSlateColor "(R=0.108477,G=1.000000,B=0.110855,A=1.000000)"))
    (else
      (Default|SetColor _arrowref (Utilities|Struct|MakeSlateColor "(R=1.000000,G=0.000000,B=0.000000,A=1.000000)")))))

(event EventBeginPlay
  (bind _returnvalue (UserInterface|CreateWidget "/Game/Widgets/Arrow.Arrow_C"))
  (bind _output_get (Variables|Default|SetArrowRef _returnvalue))
  (UserInterface|SetWidget (Variables|Default|GetWidget) _output_get)
  (bind _asmy_character (Utilities|Casting|CastTomyCharacter (Game|GetPlayerCharacter 0)))
  (Variables|Default|SetPlayerRef _asmy_character)
  (bind _asmy_game_mode (Utilities|Casting|CastTomyGameMode (Game|GetGameMode)))
  (EventDispatchers|BindEventtoStageUpdated _asmy_game_mode (delegate Custom|ChangeColor))
  (CallFunction|ChangeColor "NewEnumerator0"))

(event Collision|EventActorBeginOverlap
  (params (OtherActor :type Actor%20Object%20Reference)))

(event EventTick
  (params (DeltaSeconds :type Float%20%28single-precision%29)))

(fn ConstructionScript
  (bind _size (Variables|Widget|GetSize))
  (bind _returnvalue (Math|Conversions|ToFloat(Integer) _size))
  (Class|WidgetComponent|SetDrawSize (Variables|Default|GetWidget) (Math|Vector2D|MakeVector2D _returnvalue _returnvalue)))

(fn SetColor
  (params (Color :type Linear%20Color%20Structure))
  (Default|SetColor (Variables|Default|GetArrowRef) (Utilities|Struct|MakeSlateColor Color)))