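; Wire actor that carries a signal to its Output in a chain of connected objects and shows the link visually.
; Each tick it draws a debug line from its location to the origin of a valid Output.
; GetInput sets the line to bright green for a value of 1, dim green otherwise, then forwards the value to Output.
; An IsHead branch that would send 1 is left unconnected.
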(event EventBeginPlay
  (|CallParentFunction))

(event Collision|EventActorBeginOverlap
  (params (OtherActor :type Actor%20Object%20Reference))
  (|CallParentFunction OtherActor) ; This node is disabled and will not be called.\nDrag off pins to build functionality.
)

(event EventTick
  (params (DeltaSeconds :type Float%20%28single-precision%29))
  (bind _output (Variables|Default|GetOutput))
  (|CallParentFunction DeltaSeconds)
  (Utilities|IsValid _output
    (:Is%20Valid
      (bind _value (Default|GetOrigin _output))
      (Rendering|Debug|DrawDebugLine (Transformation|GetActorLocation) _value (Variables|WireSettings|GetColor) (Variables|WireSettings|GetDuration) (Variables|WireSettings|GetThickness)))))

(event EventGetInput
  (params (Value :type Integer))
  (bind _output (Variables|Default|GetOutput))
  (|CallParentFunction Value)
  (if (== (Variables|Default|GetValue) 1)
    (Variables|WireSettings|SetColor "(R=0.454902,G=1.000000,B=0.352941,A=1.000000)")
    (else
      (Variables|WireSettings|SetColor "(R=0.227451,G=0.498039,B=0.176471,A=1.000000)")))
  (Utilities|IsValid _output
    (:Is%20Valid
      (Default|GetInput _output (Variables|Default|GetValue)))))

(fn ConstructionScript
  (|CallParentFunction))