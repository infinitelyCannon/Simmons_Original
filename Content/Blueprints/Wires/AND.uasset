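; AND gate Blueprint for a wire-based logic system, combining any number of indexed inputs into a single output.
; GetInput stores each incoming value in the Bits array at its index, growing the array as needed, then ANDs all stored bits.
; The result is pushed immediately to the linked Output's GetInput at OutputIndex, so gates chain by event propagation without ticking.
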(event EventBeginPlay
  (|CallParentFunction) ; This node is disabled and will not be called.\nDrag off pins to build functionality.
)

(event Collision|EventActorBeginOverlap
  (params (OtherActor :type Actor%20Object%20Reference))
  (|CallParentFunction OtherActor) ; This node is disabled and will not be called.\nDrag off pins to build functionality.
)

(event EventTick
  (params (DeltaSeconds :type Float%20%28single-precision%29))
  (|CallParentFunction DeltaSeconds) ; This node is disabled and will not be called.\nDrag off pins to build functionality.
)

(event EventGetInput
  (params (Index :type Integer) (Value :type Integer))
  (bind _bits (Variables|Default|GetBits))
  (bind _output (Variables|Default|GetOutput))
  (Utilities|Array|SetArrayElem _bits Index Value true)
  (Variables|Default|SetResult (Utilities|Array|Get(acopy) _bits))
  (for _array_element (Variables|Default|GetBits)
    (Variables|Default|SetResult (Class|KismetMathLibrary|AndIntInt _array_element (Variables|Default|GetResult))))
  (Utilities|IsValid _output
    (:Is%20Valid
      (Default|GetInput _output (Variables|Default|GetOutputIndex) (Variables|Default|GetResult)))))

(fn ConstructionScript
  (|CallParentFunction))