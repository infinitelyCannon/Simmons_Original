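; NOT gate actor for a wire-based logic system, inverting the value it receives.
; GetInput stores 1 in its single-element Bits array for a zero input and 0 otherwise, then forwards that bit to the linked Output at OutputIndex if valid.
; The construction script sizes and zeroes Bits, and propagation is call-driven with no active Tick.
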(event EventBeginPlay
  (|CallParentFunction))

(event Collision|EventActorBeginOverlap
  (params (OtherActor :type Actor%20Object%20Reference))
  (|CallParentFunction OtherActor) ; This node is disabled and will not be called.\nDrag off pins to build functionality.
)

(event EventTick
  (params (DeltaSeconds :type Float%20%28single-precision%29))
  (|CallParentFunction DeltaSeconds) ; This node is disabled and will not be called.\nDrag off pins to build functionality.
)

(event EventGetInput
  (params (Index :type Integer) (Value :type Integer))
  (bind _bits (Variables|Default|GetBits))
  (bind _output (Variables|Default|GetOutput))
  (if (== Value 0)
    (Utilities|Array|SetArrayElem _bits 0 1)
    (else
      (Utilities|Array|SetArrayElem _bits 0 0)))
  (Utilities|IsValid _output
    (:Is%20Valid
      (Default|GetInput _output (Variables|Default|GetOutputIndex) (Utilities|Array|Get(acopy) (Variables|Default|GetBits))))))

(fn ConstructionScript
  (bind _bits (Variables|Default|GetBits))
  (|CallParentFunction)
  (Utilities|Array|Resize _bits 1)
  (for _index (range 0 (- (Utilities|Array|Length _bits) 1))
    (Utilities|Array|SetArrayElem (Variables|Default|GetBits) _index 0)))