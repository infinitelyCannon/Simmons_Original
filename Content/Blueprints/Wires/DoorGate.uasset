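; DoorGate is a door Blueprint from the Wires folder that opens and closes in response to an input value.
; Its GetInput event plays a timeline when the value is 1 and reverses it otherwise.
; The timeline alpha uniformly scales the Door component from full size down to zero, so the door shrinks away to open rather than moving or rotating.
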(event EventBeginPlay
  (|CallParentFunction) ; This node is disabled and will not be called.\nDrag off pins to build functionality.
)

(event Collision|EventActorBeginOverlap
  (params (OtherActor :type Actor%20Object%20Reference))
  (|CallParentFunction OtherActor) ; This node is disabled and will not be called.\nDrag off pins to build functionality.
)

(event EventTick
  (params (DeltaSeconds :type Float%20%28single-precision%29))
  (|CallParentFunction DeltaSeconds) ; This node is disabled and will not be called.\nDrag off pins to build functionality.
)

(event EventGetInput
  (params (Index :type Integer) (Value :type Integer))
  (if (== Value 1)
    (bind _alpha (Timeline|Timeline_0 Play)
      (:Update
        (Transformation|SetRelativeScale3D (Variables|Default|GetDoor) (Math|Vector|MakeVector (Math|Float|Lerp 1.0 0.0 _alpha) (Math|Float|Lerp 1.0 0.0 _alpha) (Math|Float|Lerp 1.0 0.0 _alpha)))))
    (else
      (Timeline|Timeline_0 Reverse))))

(fn ConstructionScript
  (|CallParentFunction))