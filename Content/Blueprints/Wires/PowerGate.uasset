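; PowerGate is a constant-value gate for the wire system, acting as a power source that feeds 1 or 0 into its connected wires.
; AddWire registers a wire in the Outputs array.
; GetOutput sends every registered wire a 1 when IsPositive is true and a 0 otherwise, reading no inputs.
; The event graph and construction script add no logic of their own.
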(event EventBeginPlay
  (|CallParentFunction))

(event Collision|EventActorBeginOverlap
  (params (OtherActor :type Actor%20Object%20Reference))
  (|CallParentFunction OtherActor) ; This node is disabled and will not be called.\nDrag off pins to build functionality.
)

(event EventTick
  (params (DeltaSeconds :type Float%20%28single-precision%29))
  (|CallParentFunction DeltaSeconds) ; This node is disabled and will not be called.\nDrag off pins to build functionality.
)

(fn ConstructionScript
  (|CallParentFunction))

(fn GetOutput
  (for _array_element (Variables|Default|GetOutputs)
    (Default|Send _array_element (Math|Integer|SelectInt 1 0 (Variables|Default|GetisPositive)))))

(fn AddWire
  (params (Wire :type Wire%20Spline%20Object%20Reference))
  (Utilities|Array|Add (Variables|Default|GetOutputs) Wire))