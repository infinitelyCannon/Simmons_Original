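; A wire-driven door that opens and closes according to the input value it receives through GetInput.
; An input of 1 plays the MoveDoor timeline, lerping the door from its starting relative location to a fixed height above it; any other value reverses the timeline.
; The construction script gives the Cube a dynamic text material with configurable text color, background color and letter texture.
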(event EventBeginPlay
  (|CallParentFunction)
  (Transformation|SetRelativeLocation (Variables|Default|GetCube) (Variables|Default|GetOrigin) false false)
  (bind _output_get (Variables|Default|SetStart (Variables|/Script/Engine.SceneComponent|GetRelativeLocation (Variables|Default|GetDoor))))
  (Variables|Default|SetEnd (+ _output_get "0.000000, 0,325.000000")))

(event Collision|EventActorBeginOverlap
  (params (OtherActor :type Actor%20Object%20Reference))
  (|CallParentFunction OtherActor) ; This node is disabled and will not be called.\nDrag off pins to build functionality.
)

(event EventTick
  (params (DeltaSeconds :type Float%20%28single-precision%29))
  (|CallParentFunction DeltaSeconds) ; This node is disabled and will not be called.\nDrag off pins to build functionality.
)

(event EventGetInput
  (params (Value :type Integer))
  (|CallParentFunction Value)
  (if (== Value 1)
    (bind _alpha (Timeline|MoveDoor Play)
      (:Update
        (Transformation|SetRelativeLocation (Variables|Default|GetDoor) (Math|Vector|Lerp(Vector) (Variables|Default|GetStart) (Variables|Default|GetEnd) _alpha) false false)))
    (else
      (Timeline|MoveDoor Reverse))))

(fn ConstructionScript
  (|CallParentFunction)
  (bind _returnvalue (Rendering|Material|CreateDynamicMaterialInstance "/Game/Materials/WB_Plain_Text_Inst.WB_Plain_Text_Inst" "None" :!class /Script/Engine.KismetMaterialLibrary))
  (bind _output_get (Variables|Default|SetmyMaterial _returnvalue))
  (Rendering|Material|SetVectorParameterValue _output_get "Color" (Variables|Default|GetTextColor) :!class /Script/Engine.MaterialInstanceDynamic)
  (Rendering|Material|SetVectorParameterValue (Variables|Default|GetmyMaterial) "BackgroundColor" (Variables|Default|GetBackgroundColor) :!class /Script/Engine.MaterialInstanceDynamic)
  (Rendering|Material|SetTextureParameterValue (Variables|Default|GetmyMaterial) "LetterTexture" (Variables|Default|GetTexture))
  (Rendering|Material|SetMaterial (Variables|Default|GetCube) 0 (Variables|Default|GetmyMaterial)))