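; AND_In1 is an input Blueprint for an AND gate in a wire-based logic system.
; It overrides GetInput, calling the parent version first, then checking that MyParent is valid.
; It casts MyParent to AndGate and forwards the value to that gate's ParseInput, with no other active logic of its own.
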(event EventBeginPlay
  (|CallParentFunction) ; This node is disabled and will not be called.\nDrag off pins to build functionality.
)

(event Collision|EventActorBeginOverlap
  (params (OtherActor :type Actor%20Object%20Reference))
  (|CallParentFunction OtherActor) ; This node is disabled and will not be called.\nDrag off pins to build functionality.
)

(event EventTick
  (params (DeltaSeconds :type Float%20%28single-precision%29))
  (|CallParentFunction DeltaSeconds) ; This node is disabled and will not be called.\nDrag off pins to build functionality.
)

(event EventGetInput
  (params (Value :type Integer))
  (bind _myparent (Variables|Default|GetmyParent))
  (|CallParentFunction Value)
  (Utilities|IsValid _myparent
    (:Is%20Valid
      (bind _asand_gate (Utilities|Casting|CastToAndGate _myparent))
      (Default|ParseInput _asand_gate Value))))

(fn ConstructionScript
  (|CallParentFunction))