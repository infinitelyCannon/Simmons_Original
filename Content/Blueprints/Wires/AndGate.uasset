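; AndGate is a logic gate actor that combines two inputs with AND and passes the result to a connected Output.
; ParseInput and ParseInput2 each store their value, recompute the AND and send it through GetInput if Output is valid.
; BeginPlay moves the One and Two actors to offsets relative to the gate.
; The construction script gives the cube a dynamic material with configurable colors and letter texture.
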(event EventBeginPlay
  (|CallParentFunction)
  (Transformation|SetActorLocation (Variables|Default|GetOne) (Math|Transform|TransformLocation (Transformation|GetActorTransform) (Variables|Default|GetOneVec)) false false)
  (Transformation|SetActorLocation (Variables|Default|GetTwo) (Math|Transform|TransformLocation (Transformation|GetActorTransform) (Variables|Default|GetTwoVec)) false false))

(event Collision|EventActorBeginOverlap
  (params (OtherActor :type Actor%20Object%20Reference))
  (|CallParentFunction OtherActor) ; This node is disabled and will not be called.\nDrag off pins to build functionality.
)

(event EventTick
  (params (DeltaSeconds :type Float%20%28single-precision%29))
  (|CallParentFunction DeltaSeconds) ; This node is disabled and will not be called.\nDrag off pins to build functionality.
)

(event EventParseInput
  (params (Value :type Integer))
  (bind _output (Variables|Default|GetOutput))
  (bind _output_get (Variables|Default|SetVal1 Value))
  (Variables|Default|SetValue (Class|KismetMathLibrary|AndIntInt _output_get (Variables|Default|GetVal2)))
  (Utilities|IsValid _output
    (:Is%20Valid
      (Default|GetInput _output (Variables|Default|GetValue)))))

(event EventParseInput2
  (params (Bit :type Integer))
  (bind _output (Variables|Default|GetOutput))
  (bind _output_get (Variables|Default|SetVal2 Bit))
  (Variables|Default|SetValue (Class|KismetMathLibrary|AndIntInt _output_get (Variables|Default|GetVal1)))
  (Utilities|IsValid _output
    (:Is%20Valid
      (Default|GetInput _output (Variables|Default|GetValue)))))

(fn ConstructionScript
  (|CallParentFunction)
  (bind _returnvalue (Rendering|Material|CreateDynamicMaterialInstance "/Game/Materials/WB_Plain_Text_Inst.WB_Plain_Text_Inst" "None" :!class /Script/Engine.KismetMaterialLibrary))
  (bind _output_get (Variables|Default|SetmyMaterial _returnvalue))
  (Rendering|Material|SetVectorParameterValue _output_get "Color" (Variables|Default|GetTextColor) :!class /Script/Engine.MaterialInstanceDynamic)
  (Rendering|Material|SetVectorParameterValue (Variables|Default|GetmyMaterial) "BackgroundColor" (Variables|Default|GetBackgroundColor) :!class /Script/Engine.MaterialInstanceDynamic)
  (Rendering|Material|SetTextureParameterValue (Variables|Default|GetmyMaterial) "LetterTexture" (Variables|Default|GetTexture))
  (Rendering|Material|SetMaterial (Variables|Default|GetCube) 0 (Variables|Default|GetmyMaterial)))