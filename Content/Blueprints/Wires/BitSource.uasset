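; BitSource is a wire-system actor that acts as a signal source, emitting a starting value to its connected outputs.
; On BeginPlay it sets Value from StartValue and pushes it to every entry in AllOutputs through GetInput; Resend pushes the current Value again.
; The construction script applies a dynamic material to its Cube, setting text color, background color and letter texture for its label.
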(event EventBeginPlay
  (|CallParentFunction)
  (Variables|Default|SetValue (Variables|Default|GetStartValue))
  (for _array_element (Variables|Default|GetAllOutputs)
    (Default|GetInput _array_element (Variables|Default|GetValue))))

(event Collision|EventActorBeginOverlap
  (params (OtherActor :type Actor%20Object%20Reference))
  (|CallParentFunction OtherActor) ; This node is disabled and will not be called.\nDrag off pins to build functionality.
)

(event EventTick
  (params (DeltaSeconds :type Float%20%28single-precision%29))
  (|CallParentFunction DeltaSeconds) ; This node is disabled and will not be called.\nDrag off pins to build functionality.
)

(fn ConstructionScript
  (|CallParentFunction)
  (bind _returnvalue (Rendering|Material|CreateDynamicMaterialInstance "/Game/Materials/WB_Plain_Text_Inst.WB_Plain_Text_Inst" "None" :!class /Script/Engine.KismetMaterialLibrary))
  (bind _output_get (Variables|Default|SetmyMaterial _returnvalue))
  (Rendering|Material|SetVectorParameterValue _output_get "Color" (Variables|Default|GetTextColor) :!class /Script/Engine.MaterialInstanceDynamic)
  (Rendering|Material|SetVectorParameterValue (Variables|Default|GetmyMaterial) "BackgroundColor" (Variables|Default|GetBackgroundColor) :!class /Script/Engine.MaterialInstanceDynamic)
  (Rendering|Material|SetTextureParameterValue (Variables|Default|GetmyMaterial) "LetterTexture" (Variables|Default|GetTexture))
  (Rendering|Material|SetMaterial (Variables|Default|GetCube) 0 (Variables|Default|GetmyMaterial)))

(fn Resend
  (for _array_element (Variables|Default|GetAllOutputs)
    (Default|GetInput _array_element (Variables|Default|GetValue))))