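; Spinning pickup actor that triggers either a kill or an aim action on the player character that touches it.
; Tick rotates the static mesh around yaw at a constant, frame-rate-independent speed.
; On box overlap it casts to myCharacter and, guarded by a DoOnce, calls TriggerKill or TriggerAim depending on the CanKill flag, then destroys itself.
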(event OnComponentBeginOverlap(Box)
  (params (OverlappedComponent :type Primitive%20Component%20Object%20Reference) (OtherActor :type Actor%20Object%20Reference) (OtherComp :type Primitive%20Component%20Object%20Reference) (OtherBodyIndex :type Integer) (bFromSweep :type Boolean) (SweepResult :type Hit%20Result%20Structure%20%28by%20ref%29))
  (bind _asmy_character (Utilities|Casting|CastTomyCharacter OtherActor))
  (Utilities|FlowControl|DoOnce false
    (:Completed
      (if (Variables|Default|GetcanKill)
        (Default|TriggerKill _asmy_character)
        (Actor|DestroyActor)
        (else
          (Default|TriggerAim _asmy_character)
          (Actor|DestroyActor))))))

(event EventBeginPlay)

(event Collision|EventActorBeginOverlap
  (params (OtherActor :type Actor%20Object%20Reference)))

(event EventTick
  (params (DeltaSeconds :type Float%20%28single-precision%29))
  (Transformation|AddLocalRotation (Variables|Default|GetStaticMesh) (* (Math|Rotator|MakeRotator 0.0 0.0 5e+01) DeltaSeconds) false false))

(fn ConstructionScript)