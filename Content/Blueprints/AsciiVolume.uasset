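; AsciiVolume is a box-sized post-process volume that applies an ASCII-character screen effect.
; Construction sizes the box and adds a dynamic instance of ASCII_Inst as a blendable.
; UpdateParameters pushes character, color, brightness and exposure-distance variables to the material and toggles the post process, at construction and every Tick.
; SetActive and SetRevealRadius bypass those variables, so the next Tick overwrites their changes.
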(event EventBeginPlay)

(event Collision|EventActorBeginOverlap
  (params (OtherActor :type Actor%20Object%20Reference)))

(event EventTick
  (params (DeltaSeconds :type Float%20%28single-precision%29))
  (CallFunction|UpdateParameters))

(fn ConstructionScript
  (Components|Box|SetBoxExtent (Variables|Default|GetBox) (Math|Vector|MakeVector (Variables|PostProcessSettings|GetBoxX) (Variables|PostProcessSettings|GetBoxY) (Variables|PostProcessSettings|GetBoxZ)) true)
  (bind _returnvalue (Rendering|Material|CreateDynamicMaterialInstance "/Game/TestContent/Materials/ASCII_Inst.ASCII_Inst" "None" :!class /Script/Engine.KismetMaterialLibrary))
  (bind _output_get (Variables|Default|SetMaterial _returnvalue))
  (Rendering|AddorUpdateBlendable (Variables|Default|GetPostProcess) _output_get 1.0 :!class /Script/Engine.PostProcessComponent)
  (CallFunction|UpdateParameters))

(fn UpdateParameters
  (bind _material (Variables|Default|GetMaterial))
  (bind _material_2 (Variables|Default|GetMaterial))
  (bind _material_3 (Variables|Default|GetMaterial))
  (Rendering|Material|SetScalarParameterValue _material_3 "Monochrome" (Math|Float|SelectFloat 1.0 0.0 (Variables|PostProcessSettings|GetMonochrome)) :!class /Script/Engine.MaterialInstanceDynamic)
  (Rendering|Material|SetTextureParameterValue _material_3 "CharacterImage" (Variables|PostProcessSettings|GetCharacterImage))
  (Rendering|Material|SetScalarParameterValue _material_3 "BrightnessAdjustment" (Variables|PostProcessSettings|GetBrightnessAdjustment) :!class /Script/Engine.MaterialInstanceDynamic)
  (Rendering|Material|SetScalarParameterValue _material "CharacterHeight" (Variables|PostProcessSettings|GetCharacterHeight) :!class /Script/Engine.MaterialInstanceDynamic)
  (Rendering|Material|SetScalarParameterValue _material "CharacterWidth" (Variables|PostProcessSettings|GetCharacterWidth) :!class /Script/Engine.MaterialInstanceDynamic)
  (Rendering|Material|SetScalarParameterValue _material "ColorCrunch" (Variables|PostProcessSettings|GetColorCrunch) :!class /Script/Engine.MaterialInstanceDynamic)
  (Rendering|Material|SetScalarParameterValue _material "NumberOfCharacters" (Variables|PostProcessSettings|GetNumberOfCharacters) :!class /Script/Engine.MaterialInstanceDynamic)
  (Rendering|Material|SetVectorParameterValue _material_2 "BackgroundColor" (Variables|PostProcessSettings|GetBackgroundColor) :!class /Script/Engine.MaterialInstanceDynamic)
  (Rendering|Material|SetVectorParameterValue _material_2 "ForegroundColor" (Variables|PostProcessSettings|GetForegroundColor) :!class /Script/Engine.MaterialInstanceDynamic)
  (Rendering|Material|SetScalarParameterValue (Variables|Default|GetMaterial) "ExposureDistance" (Variables|PostProcessSettings|GetExposureDistance) :!class /Script/Engine.MaterialInstanceDynamic)
  (Variables|/Script/Engine.PostProcessComponent|SetbEnabled (Variables|Default|GetPostProcess) (Variables|PostProcessSettings|GetAcivateMaterial)))

(fn SetActive
  (params (Value :type Boolean))
  (Variables|/Script/Engine.PostProcessComponent|SetbEnabled (Variables|Default|GetPostProcess) Value))

(fn SetRevealRadius
  (params (Radius :type Float%20%28single-precision%29))
  (Rendering|Material|SetScalarParameterValue (Variables|Default|GetMaterial) "ExposureDistance" Radius :!class /Script/Engine.MaterialInstanceDynamic))